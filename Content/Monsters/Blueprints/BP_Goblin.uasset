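; Goblin monster with a melee attack that damages the top-down player character and basic turrets.
; Attack spawns a slash effect at the sprite and immediately box-overlaps nearby pawns to apply fixed damage through a damage-info struct.
; The slash's animation-finished callback clears the attacking flag and signals attack end.
; It also maps walk and sprint states to movement speeds and debug-prints its element and species after spawning.
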(event `self.ReceiveBeginPlay`
  (`parent.ReceiveBeginPlay`)
  (`KismetSystemLibrary.DelayUntilNextTick`)
  (`KismetSystemLibrary.PrintString` (`|GetEnumeratorNameAsString` (`self.ElementalType`)))
  (`KismetSystemLibrary.PrintString` (`|GetEnumeratorNameAsString` (`self.Species`))))

(event `OnFinishedAnim_Event`
  (`self.OnAttackEnd`)
  (set `self.Attacking` false))

(event `/Game/Monsters/AI/BPI_MonsterAI.Attack`
  (bind _s_damageinfo (make `/Game/GameSystems/DamageSystem/S_DamageInfo` 5.0 "NewEnumerator1"))
  (bind (_returnvalue_location _returnvalue_rotation) (`KismetMathLibrary.BreakTransform` (`SceneComponent.K2_GetComponentToWorld` (`self.Sprite`))))
  (set `self.Attacking` true)
  (bind _returnvalue (`|SpawnActorFromClass` "/Game/Monsters/Blueprints/BP_Slash.BP_Slash_C" (`KismetMathLibrary.MakeTransform` _returnvalue_location _returnvalue_rotation) "Undefined" "MultiplyWithRoot" null null))
  (add `/Game/Monsters/Blueprints/BP_Slash.OnFinishedAnim` _returnvalue (delegate `OnFinishedAnim_Event`))
  (bind (_outactors _returnvalue_2) (`KismetSystemLibrary.BoxOverlapActors` (`self.K2_GetActorLocation`) (`self.Box Extent`) (`|MakeArray` "ObjectTypeQuery3" :!type "EObjectTypeQuery Enum") null (`|MakeArray` self :!type "Actor Object Reference")))
  (if _returnvalue_2
    (for _array_element _outactors
      (bind _asbp_top_down_character (cast `/Game/Character/Blueprints/BP_TopDownCharacter` _array_element)
        (:`then`
          (message `/Game/GameSystems/DamageSystem/BPI_Damageable.TakeDamage` _asbp_top_down_character _s_damageinfo self))
        (:`CastFailed`
          (bind _asbp_turret_basic (cast `/Game/Turrets_Test/Basic/BP_Turret_Basic` _array_element))
          (`/Game/GameSystems/DamageSystem/BPI_Damageable.TakeDamage` _asbp_turret_basic _s_damageinfo self))))))

(fn `SetMovementSpeed`
  (params (Speed :type "/Game/Monsters/AI/Enums/E_MovementSpeed Enum" :default "NewEnumerator0"))
  (returns (SpeedVal :type "Float (double-precision)"))
  (bind _output_get (set `CharacterMovementComponent.MaxWalkSpeed` (select `/Game/Monsters/AI/Enums/E_MovementSpeed` Speed :`NewEnumerator0` 100.0 :`NewEnumerator1` 200.0) (`self.CharacterMovement`)))
  (return _output_get))

(fn `UserConstructionScript`
  (`parent.UserConstructionScript`))