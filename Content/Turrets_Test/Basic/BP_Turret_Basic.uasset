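; Basic turret actor that deploys on spawn, takes damage and destroys itself on death.
; BeginPlay creates the health bar widget and hides the turret head for a short delay before revealing it and setting IsDeployed.
; Damage interface calls route TakeDamage and IsDead to BPC_DamageSystem, refreshing the health bar after hits.
; Most other interface functions are default-value stubs, and Get Current Health returns max health.
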(event `self.BPC_DamageSystem.OnDeath`
  (`self.K2_DestroyActor`))

(event `self.BPC_DamageSystem.OnDamageResponse`
  (params (DamageResponse :type "/Game/GameSystems/DamageSystem/E_DamageResponse Enum" :default "NewEnumerator0") (DamageCauser :type "Actor Object Reference"))
  ;[1 1 1] for hit effect (logic is handled in interface)
)

(event `self.ReceiveBeginPlay`
  (bind _bpc_damagesystem (`self.BPC_DamageSystem`))
  (bind _returnvalue (`|CreateWidget` "/Game/GameSystems/DamageSystem/WB_HealthBar.WB_HealthBar_C" null null))
  (`WidgetComponent.SetWidget` (`self.HealthBar`) _returnvalue)
  (bind _output_get (set `self.HealthBarWidgetRef` _returnvalue))
  (`/Game/GameSystems/DamageSystem/WB_HealthBar.UpdateHealthPercentage` (`self.HealthBarWidgetRef`) (`/Game/GameSystems/DamageSystem/BPC_DamageSystem.Health` _bpc_damagesystem) (`/Game/GameSystems/DamageSystem/BPC_DamageSystem.MaxHealth` _bpc_damagesystem))
  (`/Game/GameSystems/DamageSystem/WB_HealthBar.UpdateHealthPercentage` _output_get (`/Game/GameSystems/DamageSystem/BPC_DamageSystem.Health` _bpc_damagesystem) (`/Game/GameSystems/DamageSystem/BPC_DamageSystem.MaxHealth` _bpc_damagesystem))
  (`SceneComponent.SetVisibility` (`self.BP_Turret_Head`) false false)
  (`KismetSystemLibrary.Delay` 1.0)
  (set `self.IsDeployed` true)
  (`SceneComponent.SetVisibility` (`self.BP_Turret_Head`) true false))

(fn `CheckIfAttackable`
  (returns (IsAttackable :type Boolean))
  (return false))

(fn `CheckIfUnstoppableAttackable`
  (returns (IsUnstoppableAttackable :type Boolean))
  (return false))

(fn `Get Current Health`
  (returns (MaxHealth :type "Float (double-precision)"))
  (return (`/Game/GameSystems/DamageSystem/BPC_DamageSystem.MaxHealth` (`self.BPC_DamageSystem`))))

(fn `Get Max Health`
  (returns (MaxHealth :type "Float (double-precision)"))
  (return (`/Game/GameSystems/DamageSystem/BPC_DamageSystem.MaxHealth` (`self.BPC_DamageSystem`))))

(fn `GetCurrentHealth`
  (returns (Health :type "Float (double-precision)"))
  (return 0.0))

(fn `GetMaxHealth`
  (returns (MaxHealth :type "Float (double-precision)"))
  (return 0.0))

(fn `GetTeamNumber`
  (returns (TeamNumber :type Integer))
  (return 0))

(fn `Heal`
  (params (Amount :type "Float (double-precision)"))
  (returns (NewHealth :type "Float (double-precision)"))
  (return 0.0))

(fn `IsAttacking`
  (returns (Attacking :type Boolean))
  (return false))

(fn `IsDead`
  (returns (Dead :type Boolean))
  (return (`/Game/GameSystems/DamageSystem/BPC_DamageSystem.IsDead` (`self.BPC_DamageSystem`))))

(fn `TakeDamage`
  (params (DamageInfo :type "/Game/GameSystems/DamageSystem/S_DamageInfo Structure") (`Damage Causer` :type "Actor Object Reference"))
  (returns (WasDamaged :type Boolean))
  (bind _bpc_damagesystem (`self.BPC_DamageSystem`))
  (bind _wasdamaged (`/Game/GameSystems/DamageSystem/BPC_DamageSystem.TakeDamage` _bpc_damagesystem DamageInfo `Damage Causer`))
  (`/Engine/EditorBlueprintResources/StandardMacros.IsValid` _bpc_damagesystem
    (:`Is Valid`
      (`/Game/GameSystems/DamageSystem/WB_HealthBar.UpdateHealthPercentage` (`self.HealthBarWidgetRef`) (`/Game/GameSystems/DamageSystem/BPC_DamageSystem.Health` _bpc_damagesystem) (`/Game/GameSystems/DamageSystem/BPC_DamageSystem.MaxHealth` _bpc_damagesystem))
      (return _wasdamaged))))

(fn `UserConstructionScript`)