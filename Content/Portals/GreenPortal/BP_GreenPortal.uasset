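; BP_GreenPortal is a short-lived portal actor that spawns a goblin enemy.
; On BeginPlay it waits briefly, spawns a BP_Goblin running BT_Enemy_Base at its own location, sets its status flags, then destroys itself after another short delay.
; A disconnected GameManager wave-number switch remains in the graph but never runs.
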(event `self.ReceiveBeginPlay`
  (`KismetSystemLibrary.Delay` 1.0)
  (set `self.IsSpawned` true)
  (`AIBlueprintHelperLibrary.SpawnAIFromClass` "/Game/Enemies/Blueprints/BP_Goblin.BP_Goblin_C" "/Game/Enemies/AI/BehaviorTree/BT_Enemy_Base.BT_Enemy_Base" (`self.K2_GetActorLocation`) (struct) false null)
  (set `self.DoneWork` true)
  (`KismetSystemLibrary.Delay` 1.0)
  (`self.K2_DestroyActor`))

(fn `UserConstructionScript`)