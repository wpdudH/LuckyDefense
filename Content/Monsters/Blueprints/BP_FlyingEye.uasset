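; BP_FlyingEye is a flying eye monster that deals melee damage to top-down player characters and basic turrets.
; Attack box-overlaps pawns around it, damages those two types, then waits a second before clearing Attacking and signalling attack end.
; That end step runs only when the overlap finds something, so a miss leaves Attacking set.
; SetMovementSpeed scales walk or sprint speed by a multiplier, and BeginPlay prints element and species.
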(event `self.ReceiveBeginPlay`
  (`parent.ReceiveBeginPlay`)
  (`KismetSystemLibrary.DelayUntilNextTick`)
  (`KismetSystemLibrary.PrintString` (`|GetEnumeratorNameAsString` (`self.ElementalType`)))
  (`KismetSystemLibrary.PrintString` (`|GetEnumeratorNameAsString` (`self.Species`))))

(event `/Game/Monsters/AI/BPI_MonsterAI.Attack`
  (bind _s_damageinfo (make `/Game/GameSystems/DamageSystem/S_DamageInfo` 5.0 "NewEnumerator1"))
  (set `self.Attacking` true)
  (bind (_outactors _returnvalue) (`KismetSystemLibrary.BoxOverlapActors` (`self.K2_GetActorLocation`) (`self.Box Extent`) (`|MakeArray` "ObjectTypeQuery3" :!type "EObjectTypeQuery Enum") null (`|MakeArray` self :!type "Actor Object Reference")))
  (if _returnvalue
    (for _array_element _outactors
      (bind _asbp_top_down_character (cast `/Game/Character/Blueprints/BP_TopDownCharacter` _array_element)
        (:`then`
          (message `/Game/GameSystems/DamageSystem/BPI_Damageable.TakeDamage` _asbp_top_down_character _s_damageinfo self))
        (:`CastFailed`
          (bind _asbp_turret_basic (cast `/Game/Turrets_Test/Basic/BP_Turret_Basic` _array_element))
          (`/Game/GameSystems/DamageSystem/BPI_Damageable.TakeDamage` _asbp_turret_basic _s_damageinfo self))))
    (`KismetSystemLibrary.Delay` 1.0)
    (`self.OnAttackEnd`)
    (set `self.Attacking` false)))

(fn `SetMovementSpeed`
  (params (Speed :type "/Game/Monsters/AI/Enums/E_MovementSpeed Enum" :default "NewEnumerator0"))
  (returns (SpeedVal :type "Float (double-precision)"))
  (bind _output_get (set `CharacterMovementComponent.MaxWalkSpeed` (* (select `/Game/Monsters/AI/Enums/E_MovementSpeed` Speed :`NewEnumerator0` 150.0 :`NewEnumerator1` 400.0) (`self.MovementSpeedMultiplier`)) (`self.CharacterMovement`)))
  (return _output_get))

(fn `UserConstructionScript`
  (`parent.UserConstructionScript`))