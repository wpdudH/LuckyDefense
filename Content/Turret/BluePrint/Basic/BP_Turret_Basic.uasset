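; Basic turret actor that tracks enemies within its shooting range and fires projectiles at a given target.
; On BeginPlay it sizes the range sphere and marks itself deployed after a short delay.
; Sphere overlaps add and remove BP_Enemy_Base actors in an Enemies list.
; Shoot spawns a BP_Projectile carrying damage and target, holds IsShooting through a brief cooldown, then calls OnEndShoot.
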(event `self.ReceiveBeginPlay`
  (`SphereComponent.SetSphereRadius` (`self.ShootingRangeSphere`) (`self.ShootingRange`) true)
  (`KismetSystemLibrary.Delay` 1.0)
  (set `self.IsDeployed` true))

(event `self.ShootingRangeSphere.OnComponentBeginOverlap`
  (params (OverlappedComponent :type "PrimitiveComponent Object Reference") (OtherActor :type "Actor Object Reference") (OtherComp :type "PrimitiveComponent Object Reference") (OtherBodyIndex :type Integer) (bFromSweep :type Boolean) (SweepResult :type "HitResult Structure (by ref)"))
  (bind _asbp_enemy_base (cast `/Game/Monsters/Blueprints/BP_Enemy_Base` OtherActor))
  (`KismetArrayLibrary.Array_Add` (`self.Enemies`) _asbp_enemy_base))

(event `self.ShootingRangeSphere.OnComponentEndOverlap`
  (params (OverlappedComponent :type "PrimitiveComponent Object Reference") (OtherActor :type "Actor Object Reference") (OtherComp :type "PrimitiveComponent Object Reference") (OtherBodyIndex :type Integer))
  (bind _asbp_enemy_base (cast `/Game/Monsters/Blueprints/BP_Enemy_Base` OtherActor))
  (`KismetArrayLibrary.Array_RemoveItem` (`self.Enemies`) _asbp_enemy_base))

(event `Shoot`
  (params (AttackTarget :type "/Game/Monsters/Blueprints/BP_Enemy_Base Object Reference"))
  (`/Engine/EditorBlueprintResources/StandardMacros.IsValid` AttackTarget
    (:`Is Valid`
      (set `self.IsShooting` true)
      (`|SpawnActorFromClass` "/Game/Turret/BluePrint/Projectile/BP_Projectile.BP_Projectile_C" (`self.GetTransform`) "Undefined" "MultiplyWithRoot" null (`self.ProjectileDamage`) AttackTarget 1000.0 0.0 null)
      (`KismetSystemLibrary.Delay` 0.5)
      (set `self.IsShooting` false)
      (`self.On End Shoot`))))

(fn `UserConstructionScript`)