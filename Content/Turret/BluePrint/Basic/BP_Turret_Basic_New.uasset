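; Basic turret actor that tracks enemies in range, fires projectiles at a given target and is destroyed on death.
; BeginPlay creates a health bar widget, sizes the range sphere and marks the turret deployed after a delay.
; Sphere overlaps maintain the Enemies list; Shoot, not called here, spawns BP_Projectile, then signals OnEndShoot after a delay.
; GetCurrentHealth returns MaxHealth; damage response and Tick buff check are empty.
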(event `self.ReceiveBeginPlay`
  (bind _bpc_damagesystem (`self.BPC_DamageSystem`))
  (bind _returnvalue (`|CreateWidget` "/Game/GameSystems/DamageSystem/WB_HealthBar.WB_HealthBar_C" null null))
  (`WidgetComponent.SetWidget` (`self.HealthBar`) _returnvalue)
  (set `self.HealthBarWidgetRef` _returnvalue)
  (`/Game/GameSystems/DamageSystem/WB_HealthBar.UpdateHealthPercentage` (`self.HealthBarWidgetRef`) (`/Game/GameSystems/DamageSystem/BPC_DamageSystem.Health` _bpc_damagesystem) (`/Game/GameSystems/DamageSystem/BPC_DamageSystem.MaxHealth` _bpc_damagesystem))
  (`SphereComponent.SetSphereRadius` (`self.ShootingRangeSphere`) (`self.ShootingRange`) true)
  (`KismetSystemLibrary.Delay` 1.0)
  (set `self.IsDeployed` true))

(event `self.ShootingRangeSphere.OnComponentBeginOverlap`
  (params (OverlappedComponent :type "PrimitiveComponent Object Reference") (OtherActor :type "Actor Object Reference") (OtherComp :type "PrimitiveComponent Object Reference") (OtherBodyIndex :type Integer) (bFromSweep :type Boolean) (SweepResult :type "HitResult Structure (by ref)"))
  (bind _asbp_enemy_base (cast `/Game/Monsters/Blueprints/BP_Enemy_Base` OtherActor))
  (`KismetArrayLibrary.Array_Add` (`self.Enemies`) _asbp_enemy_base))

(event `self.ShootingRangeSphere.OnComponentEndOverlap`
  (params (OverlappedComponent :type "PrimitiveComponent Object Reference") (OtherActor :type "Actor Object Reference") (OtherComp :type "PrimitiveComponent Object Reference") (OtherBodyIndex :type Integer))
  (bind _asbp_enemy_base (cast `/Game/Monsters/Blueprints/BP_Enemy_Base` OtherActor))
  (`KismetArrayLibrary.Array_RemoveItem` (`self.Enemies`) _asbp_enemy_base))

(event `Shoot`
  (params (AttackTarget :type "/Game/Monsters/Blueprints/BP_Enemy_Base Object Reference"))
  (`/Engine/EditorBlueprintResources/StandardMacros.IsValid` AttackTarget
    (:`Is Valid`
      (set `self.IsShooting` true)
      (`|SpawnActorFromClass` "/Game/Turret/BluePrint/Projectile/BP_Projectile.BP_Projectile_C" (`self.GetTransform`) "Undefined" "MultiplyWithRoot" self (`self.ProjectileDamage`) AttackTarget 1000.0 0.0 self)
      (`KismetSystemLibrary.Delay` 0.5)
      (set `self.IsShooting` false)
      (`self.On End Shoot`))))

(event `self.BPC_DamageSystem.OnDeath`
  (`self.K2_DestroyActor`))

(event `self.BPC_DamageSystem.OnDamageResponse`
  (params (DamageResponse :type "/Game/GameSystems/DamageSystem/E_DamageResponse Enum" :default "NewEnumerator0") (DamageCauser :type "Actor Object Reference")))

(event `self.ReceiveTick`
  (params (DeltaSeconds :type "Float (single-precision)"))
  (if (`self.IsBuff`)
    _))

(fn `Get Current Health`
  (returns (MaxHealth :type "Float (double-precision)"))
  (return (`/Game/GameSystems/DamageSystem/BPC_DamageSystem.MaxHealth` (`self.BPC_DamageSystem`))))

(fn `Get Max Health`
  (returns (MaxHealth :type "Float (double-precision)"))
  (return (`/Game/GameSystems/DamageSystem/BPC_DamageSystem.MaxHealth` (`self.BPC_DamageSystem`))))

(fn `UserConstructionScript`)