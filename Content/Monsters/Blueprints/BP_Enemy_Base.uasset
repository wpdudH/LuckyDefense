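; Base enemy for monsters, with a sprite flipped by X velocity, an animated health bar and timed knockback, speed and damage-taken modifiers.
; TakeDamage scales damage, forwards it to the damage component and updates the bar through a Timeline lerp.
; Hit responses stun the AI, launch it from the attacker, then resume attacking, with temporary interrupt immunity.
; Death stops the AI, reports species and element to BP_WaveManager, then destroys the actor.
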(event `self.ReceiveBeginPlay`
  (bind _bpc_damagesystem (`self.BPC_DamageSystem`))
  (bind _health (`/Game/GameSystems/DamageSystem/BPC_DamageSystem.Health` _bpc_damagesystem))
  (bind _maxhealth (`/Game/GameSystems/DamageSystem/BPC_DamageSystem.MaxHealth` _bpc_damagesystem))
  (bind _returnvalue (`|CreateWidget` "/Game/GameSystems/DamageSystem/WB_HealthBar.WB_HealthBar_C" null self))
  (`WidgetComponent.SetWidget` (`self.HealthBar`) _returnvalue)
  (bind _output_get (set `self.HealthBarWidgetRef` _returnvalue))
  (`/Game/GameSystems/DamageSystem/WB_HealthBar.UpdateHealthPercentage` _output_get _health _maxhealth)
  (`/Game/GameSystems/DamageSystem/WB_HealthBar.UpdateHPTexts` (`self.HealthBarWidgetRef`) _health _maxhealth)
  (`SceneComponent.SetVisibility` (`self.HealthBar`) false false))

(event `self.ReceiveTick`
  (params (DeltaSeconds :type "Float (single-precision)"))
  (bind _x (.x (`MovementComponent.Velocity` (`self.CharacterMovement`))))
  (if (> _x 0.0)
    (`SceneComponent.K2_SetRelativeRotation` :`self` (`self.Sprite`))
    (elif (< _x 0.0)
      (`SceneComponent.K2_SetRelativeRotation` (`self.Sprite`) (struct :`Yaw` 180.0) false false))))

(event `self.BPC_DamageSystem.OnDamageResponse`
  (params (DamageResponse :type "/Game/GameSystems/DamageSystem/E_DamageResponse Enum" :default "NewEnumerator0") (DamageCauser :type "Actor Object Reference"))
  (bind _aicmonsterbase (`self.AICMonsterBase`))
  (bind _bpc_damagesystem (`self.BPC_DamageSystem`))
  (set `self.IsHit` true)
  (`Controller.StopMovement` _aicmonsterbase)
  (`/Game/Monsters/AI/AIC_Monster_Base.SetStateAsStunned` _aicmonsterbase)
  (`self.LaunchCharacter` (* (`KismetMathLibrary.GetDirectionUnitVector` (`self.K2_GetActorLocation` DamageCauser) (`self.K2_GetActorLocation`)) (`self.KnockBackMagnitude`)))
  (set `/Game/GameSystems/DamageSystem/BPC_DamageSystem.IsInterruptible` false _bpc_damagesystem)
  (`KismetSystemLibrary.Delay` 1.0)
  (set `self.IsHit` false)
  (`/Game/Monsters/AI/AIC_Monster_Base.SetStateAsAttacking` _aicmonsterbase DamageCauser)
  (`KismetSystemLibrary.Delay` 3.0)
  (set `/Game/GameSystems/DamageSystem/BPC_DamageSystem.IsInterruptible` true _bpc_damagesystem))

(event `SetKnockBackMagnitude`
  (params (KnockBackMagnitude :type "Float (double-precision)") (Duration :type "Float (double-precision)"))
  ;[1 1 1] API
  (set `self.KnockBackMagnitude` KnockBackMagnitude)
  (`KismetSystemLibrary.Delay` Duration)
  (set `self.KnockBackMagnitude` 100.0))

(event `SetMovementSpeedMultiplier`
  (params (MovementSpeedRate :type "Float (double-precision)") (Duration :type "Float (double-precision)"))
  ;[1 1 1] API
  (set `self.MovementSpeedMultiplier` MovementSpeedRate)
  (`KismetSystemLibrary.Delay` Duration)
  (set `self.MovementSpeedMultiplier` 1.0))

(event `self.BPC_DamageSystem.OnDeath`
  (`SceneComponent.SetVisibility` (`self.HealthBar`) false false)
  (bind _asaic_monster_base (cast `/Game/Monsters/AI/AIC_Monster_Base` (`self.GetController`)))
  (`Controller.StopMovement` _asaic_monster_base)
  (`BrainComponent.StopLogic` (`AIController.BrainComponent` _asaic_monster_base) "")
  (bind _returnvalue (`GameplayStatics.GetActorOfClass` "/Game/GameSystems/WaveManager/BP_WaveManager.BP_WaveManager_C"))
  (`/Game/GameSystems/WaveManager/BP_WaveManager.UpdateEnemyDeathCount` _returnvalue (make `/Game/Monsters/F_MonsterInfo` (`self.Species`) (`self.ElementalType`)))
  (`KismetSystemLibrary.Delay` 2.0)
  (`self.K2_DestroyActor`))

(event `SetTakeDamageMultiplier`
  (params (TakeDamageRate :type "Float (double-precision)") (Duration :type "Float (double-precision)"))
  ;[1 1 1] API
  (set `self.TakeDamageMultiplier` TakeDamageRate)
  (`KismetSystemLibrary.Delay` Duration)
  (set `self.TakeDamageMultiplier` 1.0))

(event `UpdateHealthbar`
  (params (DamageAmount :type "Float (double-precision)") (CurrentHealth :type "Float (double-precision)") (MaxHealth :type "Float (double-precision)"))
  (bind (_direction _damagelerpalpha) (`Timeline|Timeline` :!via `PlayFromStart`)
    (:`Update`
      (`/Game/GameSystems/DamageSystem/WB_HealthBar.UpdateHealthPercentage` (`self.HealthBarWidgetRef`) (`KismetMathLibrary.Lerp` CurrentHealth (- CurrentHealth DamageAmount) _damagelerpalpha) MaxHealth))))

(fn `CheckIfAttackable`
  (returns (IsAttackable :type Boolean))
  (return false))

(fn `CheckIfUnstoppableAttackable`
  (returns (IsUnstoppableAttackable :type Boolean))
  (return false))

(fn `GetCurrentHealth`
  (returns (Health :type "Float (double-precision)"))
  (return (`/Game/GameSystems/DamageSystem/BPC_DamageSystem.Health` (`self.BPC_DamageSystem`))))

(fn `GetMaxHealth`
  (returns (MaxHealth :type "Float (double-precision)"))
  (return (`/Game/GameSystems/DamageSystem/BPC_DamageSystem.MaxHealth` (`self.BPC_DamageSystem`))))

(fn `GetTeamNumber`
  (returns (TeamNumber :type Integer))
  (return 0))

(fn `Heal`
  (params (Amount :type "Float (double-precision)"))
  (returns (NewHealth :type "Float (double-precision)"))
  (return 0.0))

(fn `IsAttacking`
  (returns (Attacking :type Boolean))
  (return (`self.Attacking`)))

(fn `IsDead`
  (returns (Dead :type Boolean))
  (return (`/Game/GameSystems/DamageSystem/BPC_DamageSystem.IsDead` (`self.BPC_DamageSystem`))))

(fn `SetMovementSpeed`
  (params (Speed :type "/Game/Monsters/AI/Enums/E_MovementSpeed Enum" :default "NewEnumerator0"))
  (returns (SpeedVal :type "Float (double-precision)"))
  (bind _output_get (set `CharacterMovementComponent.MaxWalkSpeed` (select `/Game/Monsters/AI/Enums/E_MovementSpeed` Speed :`NewEnumerator0` 200.0 :`NewEnumerator1` 500.0 :!type "Float (single-precision)") (`self.CharacterMovement`)))
  (return _output_get))

(fn `TakeDamage`
  (params (DamageInfo :type "/Game/GameSystems/DamageSystem/S_DamageInfo Structure") (`Damage Causer` :type "Actor Object Reference"))
  (returns (WasDamaged :type Boolean))
  (bind _bpc_damagesystem (`self.BPC_DamageSystem`))
  (bind _returnvalue (* (`self.TakeDamageMultiplier`) (`.Amount_2_64864A0D4320D27C3EA14D8019B5EC9D` (break `/Game/GameSystems/DamageSystem/S_DamageInfo` DamageInfo))))
  (bind _health (`/Game/GameSystems/DamageSystem/BPC_DamageSystem.Health` _bpc_damagesystem))
  (bind _maxhealth (`/Game/GameSystems/DamageSystem/BPC_DamageSystem.MaxHealth` _bpc_damagesystem))
  (if (`KismetSystemLibrary.IsValid` _bpc_damagesystem)
    (`self.UpdateHealthbar` _returnvalue _health _maxhealth)
    (`/Engine/EditorBlueprintResources/StandardMacros.IsValid` _bpc_damagesystem
      (:`Is Valid`
        (bind _wasdamaged (`/Game/GameSystems/DamageSystem/BPC_DamageSystem.TakeDamage` _bpc_damagesystem (make `/Game/GameSystems/DamageSystem/S_DamageInfo` _returnvalue) `Damage Causer`))
        (`/Game/GameSystems/DamageSystem/WB_HealthBar.UpdateHPTexts` (`self.HealthBarWidgetRef`) _health _maxhealth)
        (if (not (`/Game/GameSystems/DamageSystem/BPC_DamageSystem.IsDead` (`self.BPC_DamageSystem`)))
          (`SceneComponent.SetVisibility` (`self.HealthBar`) true false))
        (return _wasdamaged)))))

(fn `UserConstructionScript`)