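; BP_Assist_Turret is a support turret that buffs the damage of attack turrets within its range.
; When a valid actor enters its Sphere, it resizes the sphere to AssistRange and adds any BP_Turret1_Head to the Turrets array.
; The loop applies a flat ProjectileDamage increase to the entering head once per array entry, so the bonus grows with the array, and sets IsBuff.
; No logic removes the buff.
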(event `self.Sphere.OnComponentBeginOverlap`
  (params (OverlappedComponent :type "PrimitiveComponent Object Reference") (OtherActor :type "Actor Object Reference") (OtherComp :type "PrimitiveComponent Object Reference") (OtherBodyIndex :type Integer) (bFromSweep :type Boolean) (SweepResult :type "HitResult Structure (by ref)"))
  (bind _turrets (`self.Turrets`))
  (`/Engine/EditorBlueprintResources/StandardMacros.IsValid` OtherActor
    (:`Is Valid`
      (`SphereComponent.SetSphereRadius` (`self.Sphere`) (`self.Assist Range`) true)
      (bind _asbp_turret_1_head (cast `/Game/Turret/BluePrint/Head/BP_Turret1_Head` OtherActor))
      (`KismetArrayLibrary.Array_Add` _turrets _asbp_turret_1_head)
      (for _ _turrets
        (set `/Game/Turret/BluePrint/Head/BP_Turret1_Head.ProjectileDamage` (+ (`/Game/Turret/BluePrint/Head/BP_Turret1_Head.ProjectileDamage` _asbp_turret_1_head) 30.0) _asbp_turret_1_head)
        (if (not (`/Game/Turret/BluePrint/Head/BP_Turret1_Head.IsBuff` _asbp_turret_1_head))
          (set `/Game/Turret/BluePrint/Head/BP_Turret1_Head.IsBuff` true _asbp_turret_1_head))))))

(fn `UserConstructionScript`
  (`parent.UserConstructionScript`))