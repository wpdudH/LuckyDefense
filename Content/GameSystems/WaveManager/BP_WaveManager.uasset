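; Wave manager that runs data-driven enemy waves around BP_Core.
; Reads the GameManager's wave number, looks up its DT_Waves row and spawns a BP_GreenPortal per monster at random navigable points near the core.
; Each wave starts a duration timer with a countdown widget; an overdue check can broadcast OnStartNextWave, and NextWave advances while rows remain.
; Spawn points are collected, but their SpawnEnemy path is unused.
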(event `self.ReceiveBeginPlay`
  (add `self.OnStartNextWave` (`|CreateDelegate` :!event `NextWave`))
  (bind _returnvalue (`|CreateWidget` "/Game/UI/WaveInfo/WB_CombatStatus.WB_CombatStatus_C"))
  (set `self.CombatStatusWidget` _returnvalue)
  (bind _outactors (`GameplayStatics.GetAllActorsOfClass` "/Game/Monsters/Blueprints/BP_EnemySpawnPoint.BP_EnemySpawnPoint_C"))
  (for _array_element _outactors
    (`KismetArrayLibrary.Array_Add` (`self.EnemySpawnPoints`) _array_element))
  (`self.StartWave`))

(event `UpdateCombatStatus`)

(event `CheckIfWaveOverdue`
  (bind _asgame_manager (cast `/Game/GameSystems/GameManager/GameManager` (`GameplayStatics.GetGameInstance`)))
  (bind _wavenumber (`/Game/GameSystems/GameManager/GameManager.GetWaveNumber` _asgame_manager))
  (if (== _wavenumber (`self.TempWaveNum`))
    (`self.OnStartNextWave`)))

(event `NextWave`
  (bind _waveexists (`self.IncrementWaveNumber`))
  (if _waveexists
    (`self.StartWave`)))

(fn `IncrementWaveNumber`
  (returns (WaveExists :type Boolean))
  (bind _asgame_manager (cast `/Game/GameSystems/GameManager/GameManager` (`GameplayStatics.GetGameInstance`)))
  (bind _wavenumber (`/Game/GameSystems/GameManager/GameManager.GetWaveNumber` _asgame_manager))
  (bind _returnvalue (+ _wavenumber 1))
  (`/Game/GameSystems/GameManager/GameManager.SetWaveNumber` _asgame_manager _returnvalue)
  (`|GetDataTableRow` "/Game/GameSystems/GameManager/DT_Waves.DT_Waves" (`KismetStringLibrary.Conv_StringToName` (`KismetStringLibrary.Conv_IntToString` _returnvalue))
    (:`then`
      (return true))
    (:`RowNotFound`
      (return false))))

(fn `SpawnEnemy`
  (params (MonsterInfo :type "/Game/Monsters/F_MonsterInfo Structure"))
  (`|SpawnActorFromClass` "/Game/Portals/GreenPortal/BP_GreenPortal.BP_GreenPortal_C" (`KismetMathLibrary.MakeTransform` (`self.K2_GetActorLocation` (`KismetArrayLibrary.Array_Random` (`self.EnemySpawnPoints`)))) "Undefined" "MultiplyWithRoot" null MonsterInfo null))

(fn `SpawnEnemyAtRandPos`
  (params (SpawnRadius :type "Float (double-precision)") (MonsterInfo :type "/Game/Monsters/F_MonsterInfo Structure"))
  (bind _returnvalue (`GameplayStatics.GetActorOfClass` "/Game/Core/BP_Core.BP_Core_C"))
  (bind _randomlocation (`NavigationSystemV1.K2_GetRandomLocationInNavigableRadius` (`self.K2_GetActorLocation` _returnvalue) SpawnRadius null null))
  (`|SpawnActorFromClass` "/Game/Portals/GreenPortal/BP_GreenPortal.BP_GreenPortal_C" (`KismetMathLibrary.MakeTransform` _randomlocation) "Undefined" "MultiplyWithRoot" null MonsterInfo null))

(fn `StartWave`
  (bind _asgame_manager (cast `/Game/GameSystems/GameManager/GameManager` (`GameplayStatics.GetGameInstance`)))
  (bind _wavenumber (`/Game/GameSystems/GameManager/GameManager.GetWaveNumber` _asgame_manager))
  (set `self.TempWaveNum` _wavenumber)
  (bind _returnvalue (`|GetDataTableRow` "/Game/GameSystems/GameManager/DT_Waves.DT_Waves" (`KismetStringLibrary.Conv_StringToName` (`KismetStringLibrary.Conv_IntToString` _wavenumber)))
    (:`then`
      (bind (_wavenumber_2 _monsters _spawnradius _duration) (break `/Game/GameSystems/GameManager/S_Waves` _returnvalue))
      (for _index (range (`KismetArrayLibrary.Array_Length` _monsters))
        (`self.SpawnEnemyAtRandPos` 700.0 (`|GetArrayItem` _monsters _index)))
      (`KismetSystemLibrary.K2_SetTimerDelegate` (`|CreateDelegate` :!event `CheckIfWaveOverdue`) _duration)
      (bind _returnvalue_2 (`|CreateWidget` "/Game/UI/WaveInfo/WB_NextWaveTimer.WB_NextWaveTimer_C" null _duration))
      (bind _output_get (set `self.NextWaveTimerWidget` _returnvalue_2))
      (`UserWidget.AddToViewport` _output_get 0))))

(fn `UpdateEnemyDeathCount`
  (params (MonsterInfo :type "/Game/Monsters/F_MonsterInfo Structure"))
  (`KismetArrayLibrary.Array_Add` (`self.SpawnedEnemies`) MonsterInfo))

(fn `UserConstructionScript`)