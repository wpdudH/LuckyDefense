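; BP_BloodCircle is a damage-over-time area skill that hurts enemies for about five seconds, then destroys itself.
; BeginPlay runs SpawnSkill and applies an initial hit to TargetList with no target type.
; A looping half-second timer re-queries CheckTarget, damages the "Enemy" type and tracks elapsed time until expiry.
; Damage goes through the parent's DamageToTarget, which the override simply forwards to.
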(event `self.ReceiveBeginPlay`
  (`parent.ReceiveBeginPlay`)
  (`self.Spawn Skill`)
  (`self.DamageToTarget` (`self.TargetList`) "" 5.0)
  (`KismetSystemLibrary.K2_SetTimerDelegate` (delegate `TakeDamage`) 0.5 true))

(event `TakeDamage`
  (if (< (`self.ElapsedTime`) 5.0)
    (bind _outactors (`self.CheckTarget`))
    (`self.DamageToTarget` _outactors "Enemy" 5.0)
    (set `self.ElapsedTime` (+ (`self.ElapsedTime`) 0.5))
    (else
      (`self.K2_DestroyActor`))))

(fn `DamageToTarget`
  (params (Target :type "Array of Actor Object Reference (by ref)") (TargetType :type String) (DamageAmount :type "Float (double-precision)"))
  (`parent.DamageToTarget` Target TargetType DamageAmount)
  (return))

(fn `UserConstructionScript`
  (`parent.UserConstructionScript`))