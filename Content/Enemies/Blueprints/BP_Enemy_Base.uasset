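; Base 2D sprite enemy character that takes damage, attacks the player and flips its sprite to face horizontal movement.
; BPCDamageSystem holds health and death state, exposed through damage, team and movement functions (some stubbed), and initializes a widget health bar.
; Attack spawns a BP_Slash effect and immediately damages BP_TopDownCharacter actors in a box overlap.
; The slash's animation-finished event destroys it, fires OnAttackEnd and clears the attacking flag.
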(event `self.ReceiveBeginPlay`
  (bind _bpc_damagesystem (`self.BPC_DamageSystem`))
  (bind _returnvalue (`|CreateWidget` "/Game/GameSystems/DamageSystem/W_HealthBar.W_HealthBar_C" null self))
  (`WidgetComponent.SetWidget` (`self.HealthBar`) _returnvalue)
  (bind _output_get (set `self.HealthBarWidgetRef` _returnvalue))
  (`/Game/GameSystems/DamageSystem/W_HealthBar.UpdateHealthPercentage` (`self.HealthBarWidgetRef`) (`/Game/GameSystems/DamageSystem/BPC_DamageSystem.Health` _bpc_damagesystem) (`/Game/GameSystems/DamageSystem/BPC_DamageSystem.MaxHealth` _bpc_damagesystem))
  (`/Game/GameSystems/DamageSystem/W_HealthBar.UpdateHealthPercentage` _output_get (`/Game/GameSystems/DamageSystem/BPC_DamageSystem.Health` _bpc_damagesystem) (`/Game/GameSystems/DamageSystem/BPC_DamageSystem.MaxHealth` _bpc_damagesystem)))

(event `self.ReceiveTick`
  (params (DeltaSeconds :type "Float (single-precision)"))
  (bind _x (.x (`MovementComponent.Velocity` (`self.CharacterMovement`))))
  (if (> _x 0.0)
    (`SceneComponent.K2_SetRelativeRotation` :`self` (`self.Sprite`))
    (elif (< _x 0.0)
      (`SceneComponent.K2_SetRelativeRotation` (`self.Sprite`) (struct :`Yaw` 180.0) false false))))

(event `OnFinishedAnim_Event`
  (`self.K2_DestroyActor` (stale `Attack` _returnvalue))
  (`self.OnAttackEnd`)
  (set `self.Attacking` false))

(event `Attack`
  (bind (_returnvalue_location _returnvalue_rotation) (`KismetMathLibrary.BreakTransform` (`SceneComponent.K2_GetComponentToWorld` (`self.Sprite`))))
  (set `self.Attacking` true)
  (bind _returnvalue (`|SpawnActorFromClass` "/Game/Enemies/Blueprints/BP_Slash.BP_Slash_C" (`KismetMathLibrary.MakeTransform` _returnvalue_location _returnvalue_rotation) "Undefined" "MultiplyWithRoot" null null))
  (add `/Game/Enemies/Blueprints/BP_Slash.OnFinishedAnim` _returnvalue (delegate `OnFinishedAnim_Event`))
  (bind (_outactors _returnvalue_2) (`KismetSystemLibrary.BoxOverlapActors` (`self.K2_GetActorLocation`) (`self.Box Extent`) (`|MakeArray` "ObjectTypeQuery3" :!type "EObjectTypeQuery Enum") null (`|MakeArray` self :!type "Actor Object Reference")))
  (if _returnvalue_2
    (for _array_element _outactors
      (bind _asbp_top_down_character (cast `/Game/Character/Blueprints/BP_TopDownCharacter` _array_element))
      (message `/Game/GameSystems/DamageSystem/BPI_Damageable.TakeDamage` _asbp_top_down_character (make `/Game/GameSystems/DamageSystem/S_DamageInfo` 5.0 "NewEnumerator1") self)
      (`KismetSystemLibrary.PrintString` (`KismetSystemLibrary.GetDisplayName` _asbp_top_down_character)))))

(fn `CheckIfAttackable`
  (returns (IsAttackable :type Boolean))
  (return false))

(fn `CheckIfUnstoppableAttackable`
  (returns (IsUnstoppableAttackable :type Boolean))
  (return false))

(fn `GetCurrentHealth`
  (returns (Health :type "Float (double-precision)"))
  (return (`/Game/GameSystems/DamageSystem/BPC_DamageSystem.Health` (`self.BPC_DamageSystem`))))

(fn `GetMaxHealth`
  (returns (MaxHealth :type "Float (double-precision)"))
  (return (`/Game/GameSystems/DamageSystem/BPC_DamageSystem.MaxHealth` (`self.BPC_DamageSystem`))))

(fn `GetTeamNumber`
  (returns (TeamNumber :type Integer))
  (return 0))

(fn `Heal`
  (params (Amount :type "Float (double-precision)"))
  (returns (NewHealth :type "Float (double-precision)"))
  (return 0.0))

(fn `IsAttacking`
  (returns (Attacking :type Boolean))
  (return (`self.Attacking`)))

(fn `IsDead`
  (returns (Dead :type Boolean))
  (return (`/Game/GameSystems/DamageSystem/BPC_DamageSystem.IsDead` (`self.BPC_DamageSystem`))))

(fn `SetMovementSpeed`
  (params (Speed :type "/Game/Enemies/AI/Enums/E_MovementSpeed Enum" :default "NewEnumerator0"))
  (returns (SpeedVal :type "Float (double-precision)"))
  (bind _output_get (set `CharacterMovementComponent.MaxWalkSpeed` (select `/Game/Enemies/AI/Enums/E_MovementSpeed` Speed :`NewEnumerator0` 200.0 :`NewEnumerator1` 500.0 :!type "Float (single-precision)") (`self.CharacterMovement`)))
  (return _output_get))

(fn `TakeDamage`
  (params (DamageInfo :type "/Game/GameSystems/DamageSystem/S_DamageInfo Structure") (`Damage Causer` :type "Actor Object Reference"))
  (returns (WasDamaged :type Boolean))
  (bind _wasdamaged (`/Game/GameSystems/DamageSystem/BPC_DamageSystem.TakeDamage` (`self.BPC_DamageSystem`) DamageInfo `Damage Causer`))
  (return _wasdamaged))

(fn `UserConstructionScript`)