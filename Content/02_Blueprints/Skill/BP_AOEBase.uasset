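; BP_AOEBase is an area-of-effect skill base that finds pawns around a spawn position and offers effect helpers for them.
; SpawnSkill draws a debug sphere and stores class-filtered sphere-overlap results in TargetList, optionally ignoring the instigator; CheckTarget returns the same query.
; Damage and heal helpers branch on Enemy, Character or Turret, but player damage is zero and heal loops lack array inputs.
; Knockback, speed and attenuation helpers are unfinished stubs.
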(event `self.ReceiveTick`
  (params (DeltaSeconds :type "Float (single-precision)")))

(event `Spawn Skill`
  (`KismetSystemLibrary.DrawDebugSphere` (`self.Spawn Pos`) (`self.Skill Range`) 12 (struct :`G` 1.0 :`B` 0.337505 :`A` 1.0) 1000.0 2.0)
  (bind _outactors (`KismetSystemLibrary.SphereOverlapActors` (`self.Spawn Pos`) (`self.Skill Range`) (`|MakeArray` "ObjectTypeQuery3" :!type "EObjectTypeQuery Enum") (`self.Target Actor Class`) (select `bool` (`self.Ignore Instigator`) :`true` (`|MakeArray` (`self.GetInstigator`)))))
  (set `self.TargetList` _outactors))

(fn `CheckTarget`
  (returns (OutActors :type "Array of Actor Object Reference"))
  (bind _outactors (`KismetSystemLibrary.SphereOverlapActors` (`self.Spawn Pos`) (`self.Skill Range`) (`|MakeArray` "ObjectTypeQuery3" :!type "EObjectTypeQuery Enum") (`self.Target Actor Class`) (select `bool` (`self.Ignore Instigator`) :`true` (`|MakeArray` (`self.GetInstigator`)))))
  (return _outactors))

(fn `DamageToTarget`
  (params (Target :type "Array of Actor Object Reference") (TargetType :type String) (DamageAmount :type "Float (double-precision)"))
  (bind _returnvalue (`GameplayStatics.GetPlayerCharacter` 0))
  (switch `string` TargetType
    (:`Enemy`
      (for _array_element Target
        (bind _asbp_enemy_base (cast `/Game/Monsters/Blueprints/BP_Enemy_Base` _array_element))
        (message `/Game/GameSystems/DamageSystem/BPI_Damageable.TakeDamage` _asbp_enemy_base (make `/Game/GameSystems/DamageSystem/S_DamageInfo` (`local.DamageAmount`) "NewEnumerator2") (`GameplayStatics.GetPlayerCharacter` 0))))
    (:`Character`
      (message `/Game/GameSystems/DamageSystem/BPI_Damageable.TakeDamage` _returnvalue (make `/Game/GameSystems/DamageSystem/S_DamageInfo` 0.0 "NewEnumerator2") _returnvalue))
    (:`Turret`
      (for _array_element_2 Target
        (bind _asbp_turret_base (cast `/Game/Turret/BluePrint/BP_Turret_Base` _array_element_2))
        (message `/Game/GameSystems/DamageSystem/BPI_Damageable.TakeDamage` _asbp_turret_base (make `/Game/GameSystems/DamageSystem/S_DamageInfo` (`local.DamageAmount`) "NewEnumerator2") (`GameplayStatics.GetPlayerCharacter` 0))))))

(fn `HealToTarget`
  (params (Target :type "Array of Actor Object Reference") (TargetType :type String) (HealAmount :type "Float (double-precision)"))
  (switch `string` TargetType
    (:`Enemy`
      (for _array_element _
        (bind _asbp_enemy_base (cast `/Game/Monsters/Blueprints/BP_Enemy_Base` _array_element))
        (`/Game/GameSystems/DamageSystem/BPI_Damageable.Heal` _asbp_enemy_base (`local.HealAmount`))))
    (:`Character`
      (message `/Game/GameSystems/DamageSystem/BPI_Damageable.Heal` (`GameplayStatics.GetPlayerCharacter` 0) (`local.HealAmount`)))
    (:`Turret`
      (for _array_element_2 _
        (bind _asbp_turret_base (cast `/Game/Turret/BluePrint/BP_Turret_Base` _array_element_2))
        (message `/Game/GameSystems/DamageSystem/BPI_Damageable.Heal` _asbp_turret_base (`local.HealAmount`))))))

(fn `KnockBackToTarget`
  (params (Target :type "Array of Actor Object Reference") (TargetType :type String) (KnockBackAmount :type "Float (double-precision)"))
  (locals (KnockBackAmount :type "Float (double-precision)"))
  (switch `string` TargetType
    (:`Enemy`
      (for _array_element _
        (cast `/Game/Monsters/Blueprints/BP_Enemy_Base` _array_element)))
    (:`Turret`
      (for _array_element_2 _
        (cast `/Game/Turret/BluePrint/BP_Turret_Base` _array_element_2)))))

(fn `SetTargetAttenuation`
  (params (Target :type "Array of Actor Object Reference") (TargetType :type String) (SpeedAmount :type "Float (double-precision)") (ApplyTime :type "Float (double-precision)")))

(fn `SetTargetSpeed`
  (params (Target :type "Array of Actor Object Reference") (TargetType :type String) (SpeedAmount :type "Float (double-precision)") (ApplyTime :type "Float (double-precision)"))
  (switch `string` TargetType
    (:`Enemy`
      (for _array_element _
        (cast `/Game/Monsters/Blueprints/BP_Enemy_Base` _array_element)))
    (:`Turret`
      (for _array_element_2 _
        (cast `/Game/Turret/BluePrint/BP_Turret_Base` _array_element_2)))))

(fn `UserConstructionScript`)