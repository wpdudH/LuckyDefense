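; Ability system component that runs a wave-based roulette, pausing the game and showing randomly drawn ability choices in a job/ability thumbnail widget.
; Wave 1 draws from the full ID pool and switches to UI-only input; waves 2 and 3 first strip ToolNBuffList IDs by index.
; Other waves use MixRoulette, which adds a fixed ID 0 unless IsSecondJob.
; Draws avoid repeats by removing picks from a shrinking list.
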(event `StartRoulette`
  (params (WaveNumber :type Integer))
  (`GameplayStatics.SetGamePaused` true)
  (switch `int` WaveNumber
    (:`Default`
      (bind _randnumlist (`self.MixRoulette`))
      (bind _output_get (set `self.RandNumberList` _randnumlist))
      (bind _returnvalue (`|CreateWidget` "/Game/UI/Ability/WBP_JobAbilityThumbnail.WBP_JobAbilityThumbnail_C" null _output_get))
      (`UserWidget.AddToViewport` _returnvalue 0))
    (:`1`
      (bind _randnumber (`self.FirstRoulette`))
      (bind _output_get_2 (set `self.RandNumberList` _randnumber))
      (bind _returnvalue_2 (`|CreateWidget` "/Game/UI/Ability/WBP_JobAbilityThumbnail.WBP_JobAbilityThumbnail_C" null _output_get_2))
      (bind _output_get_3 (set `self.AbilityWidget` _returnvalue_2))
      (`UserWidget.AddToViewport` _output_get_3 0)
      (`WidgetBlueprintLibrary.SetInputMode_UIOnlyEx` (`GameplayStatics.GetPlayerController` 0) (`self.AbilityWidget`)))
    (:`2`
      (bind _randnumberlist (`self.ToolNBuffOnlyRoulette` 2 :!label _label))
      (bind _output_get_4 (set `self.RandNumberList` _randnumberlist))
      (bind _returnvalue_3 (`|CreateWidget` "/Game/UI/Ability/WBP_JobAbilityThumbnail.WBP_JobAbilityThumbnail_C" null _output_get_4))
      (`UserWidget.AddToViewport` _returnvalue_3 0))
    (:`3`
      (goto _label))))

(fn `CompareTwoNumber`
  (params (Current :type Integer) (Previous :type Integer))
  (if (> Current Previous)
    _))

(fn `FirstRoulette`
  (returns (RandNumber :type "Array of Integer"))
  (locals (NumberList :type "Array of Integer") (range :type Integer :default 8) (RandomNumber :type "Array of Integer") (crack :type Integer))
  (for _index (range 14)
    (`KismetArrayLibrary.Array_Add` (`local.NumberList`) _index))
  (for _ (range 3)
    (bind _output_get (set `local.crack` (`KismetMathLibrary.RandomIntegerInRange` 0 (`local.range`))))
    (`KismetArrayLibrary.Array_Add` (`local.RandomNumber`) (`|GetArrayItem` (`local.NumberList`) _output_get))
    (`KismetArrayLibrary.Array_Remove` (`local.NumberList`) (`local.crack`))
    (set `local.range` (- (`local.range`) 1)))
  (return (`local.RandomNumber`)))

(fn `GenerateRandomNumber`)

(fn `MixRoulette`
  (returns (RandNumList :type "Array of Integer"))
  (locals (RandNumber :type "Array of Integer"))
  (if (`self.IsSecondJob`)
    (bind _randnumberlist (`self.ToolNBuffOnlyRoulette` 2))
    (return _randnumberlist)
    (else
      (bind _randnumberlist_2 (`self.ToolNBuffOnlyRoulette` 1))
      (bind _output_get (set `local.RandNumber` _randnumberlist_2))
      (`KismetArrayLibrary.Array_Add` _output_get)
      (return (`local.RandNumber`)))))

(fn `ToolNBuffOnlyRoulette`
  (params (`Index Number` :type Integer))
  (returns (RandNumberList :type "Array of Integer"))
  (locals (RandNumber :type "Array of Integer") (NumberList :type "Array of Integer") (Range :type Integer :default 13) (crack :type Integer))
  (for _index (range 14)
    (`KismetArrayLibrary.Array_Add` (`local.NumberList`) _index))
  (for _array_element (`self.ToolNBuffList`)
    (`KismetArrayLibrary.Array_Remove` (`local.NumberList`) (`.ID_8_E5059BA94DE516D39F57799BC2537393` (break `/Game/GameSystems/AbilitySystem/ST_ToolNBuff` _array_element)))
    (set `local.Range` (- (`local.Range`) 1)))
  (for _ (range (+ (`local.Index Number`) 1))
    (bind _output_get (set `local.crack` (`KismetMathLibrary.RandomIntegerInRange` 0 (`local.Range`))))
    (`KismetArrayLibrary.Array_Add` (`local.RandNumber`) (`|GetArrayItem` (`local.NumberList`) _output_get))
    (`KismetArrayLibrary.Array_Remove` (`local.NumberList`) (`local.crack`))
    (set `local.Range` (- (`local.Range`) 1)))
  (return (`local.RandNumber`)))